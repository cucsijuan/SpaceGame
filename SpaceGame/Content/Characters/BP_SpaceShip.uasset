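; Player-controlled spaceship that flies, fires a laser and switches between cockpit and external cameras.
; Input axes feed roll, yaw, pitch and throttle to SpaceMovement, while Shoot starts and stops BPLaserBeam along the external camera's forward vector.
; Each tick, HandleFXs sets the thrust color on both engines' dynamic materials based on velocity.
; Impulse thrust and timer-gated rudder logic remain but are not wired to input.
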(event `self.ReceiveBeginPlay`
  (bind _returnvalue (`PrimitiveComponent.CreateDynamicMaterialInstance` (`self.EngineLeft`) 0 "/Game/Materials/MI_EngineThrust.MI_EngineThrust" "None"))
  (set `self.MD_EngineL` _returnvalue)
  (bind _returnvalue_2 (`PrimitiveComponent.CreateDynamicMaterialInstance` (`self.EngineRight`) 0 "/Game/Materials/MI_EngineThrust.MI_EngineThrust" "None"))
  (set `self.MD_EngineR` _returnvalue_2))

(event `self.ReceiveTick`
  (params (DeltaSeconds :type "Float (single-precision)"))
  (`self.HandleFXs`))

(event `InputAction|Shoot`
  (params (Key :type "Key Structure"))
  (bind _bp_laserbeam (`self.BP_LaserBeam`))
  (bind _externalcamera (`self.ExternalCamera`))
  (:`Pressed`
    (`/Game/Weapons/BP_LaserBeam.ShootLaser` _bp_laserbeam (`SceneComponent.K2_GetComponentLocation` _externalcamera) (`SceneComponent.GetForwardVector` _externalcamera)))
  (:`Released`
    (`/Game/Weapons/BP_LaserBeam.StopLaser` _bp_laserbeam)))

(event `InputAction|ChangeCameraView`
  (params (Key :type "Key Structure"))
  (bind _cockpitcamera (`self.CockpitCamera`))
  (bind _externalcamera (`self.ExternalCamera`))
  (:`Pressed`
    (`/Engine/EditorBlueprintResources/StandardMacros.FlipFlop`
      (:`A`
        (`ActorComponent.Activate` _cockpitcamera false)
        (`ActorComponent.Deactivate` _externalcamera))
      (:`B`
        (`ActorComponent.Activate` _externalcamera false)
        (`ActorComponent.Deactivate` _cockpitcamera)))))

(event `InputAxis|Roll`
  (params (AxisValue :type "Float (single-precision)"))
  (`SpaceMovementComponent.SetRollThrow` (`self.SpaceMovement`) AxisValue))

(event `InputAxis|Yaw`
  (params (AxisValue :type "Float (single-precision)"))
  (`SpaceMovementComponent.SetSteeringThrow` (`self.SpaceMovement`) AxisValue))

(event `InputAxis|Pitch`
  (params (AxisValue :type "Float (single-precision)"))
  (`SpaceMovementComponent.SetPitchThrow` (`self.SpaceMovement`) AxisValue))

(event `InputAxis|EngineThrust`
  (params (AxisValue :type "Float (single-precision)"))
  (`SpaceMovementComponent.SetThrottle` (`self.SpaceMovement`) AxisValue))

(event `CustomEvent_0`
  (`KismetSystemLibrary.K2_ClearAndInvalidateTimerHandle` (`self.RudderTimerhandle`)))

(fn `HandleFXs`
  (bind _returnvalue (`SpaceMovementComponent.GetVelocity` (`self.SpaceMovement`)))
  (bind _returnvalue_2 (`KismetMathLibrary.VSize` _returnvalue))
  (if (== _returnvalue_2 0.0)
    (`MaterialInstanceDynamic.SetVectorParameterValue` (`self.MD_EngineL`) "Thrust" (struct :`R` 0.047059 :`G` 0.098039 :`B` 0.043137 :`A` 1.0))
    (`MaterialInstanceDynamic.SetVectorParameterValue` (`self.MD_EngineR`) "Thrust" (struct :`R` 0.047059 :`G` 0.098039 :`B` 0.043137 :`A` 1.0))
    (else
      (bind _returnvalue_3 (`KismetMathLibrary.LinearColorLerp` (struct :`R` 0.047059 :`G` 0.098039 :`B` 0.043137 :`A` 1.0) (struct :`R` 1.0 :`B` 0.154889 :`A` 1.0) (`KismetMathLibrary.Abs` (/ 0.0 _returnvalue_2))))
      (`MaterialInstanceDynamic.SetVectorParameterValue` (`self.MD_EngineL`) "Thrust" _returnvalue_3)
      (`MaterialInstanceDynamic.SetVectorParameterValue` (`self.MD_EngineR`) "Thrust" _returnvalue_3))))

(fn `HandleRudderChange`
  (params (input :type "Float (double-precision)") (Delegate :type Delegate))
  (locals (LastThrustMod :type "Float (double-precision)"))
  (bind _returnvalue (+ (`self.EngineThrustMod`) (* input (* (`GameplayStatics.GetWorldDeltaSeconds`) (`self.RudderSensitivity`)))))
  (if (not (`KismetSystemLibrary.K2_IsValidTimerHandle` (`self.RudderTimerhandle`)))
    (set `local.LastThrustMod` (`self.EngineThrustMod`))
    (if (> _returnvalue 0.0)
      (set `self.EngineThrustMod` 0.0)
      (else
        (bind _output_get (set `self.EngineThrustMod` (select `bool` (< _returnvalue 0.0) :`false` _returnvalue :`true` 0.0)))
        (if (and (`KismetMathLibrary.NearlyEqual_FloatFloat` _output_get 0.0 0.1) (!= (`local.LastThrustMod`) 0.0))
          (set `self.EngineThrustMod` 0.0)
          (bind _returnvalue_2 (`KismetSystemLibrary.K2_SetTimerDelegate` Delegate 0.15))
          (set `self.RudderTimerhandle` _returnvalue_2))))))

(fn `ThrustMainEngines`
  (`PrimitiveComponent.AddImpulse` (`self.StaticMesh`) (* (`KismetMathLibrary.GetForwardVector` (`SceneComponent.K2_GetComponentRotation` (`self.RootDirectionArrow`))) (* (`self.EngineThrustMod`) 0.0)) "None" false))

(fn `UserConstructionScript`)