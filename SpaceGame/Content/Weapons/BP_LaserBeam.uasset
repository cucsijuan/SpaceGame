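; Laser beam weapon that fires a hitscan trace from the camera and shows a particle beam to whatever it hits.
; ShootLaser line traces up to WeaponRange, ignoring the owner, with debug draw and a print of the hit actor.
; On a hit, it attaches an emitter to the owner's root, setting owner and hit actor as beam source and target parameters.
; StopLaser destroys the stored emitter; no damage is applied.
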(fn `ShootLaser`
  (params (CameraLocation :type "Vector Structure") (CameraforwardVector :type "Vector Structure"))
  (bind (_outhit _returnvalue) (`KismetSystemLibrary.LineTraceSingle` CameraLocation (+ CameraLocation (* CameraforwardVector (`self.WeaponRange`))) "TraceTypeQuery1" false (`|MakeArray` (`self.GetOwner`)) "Persistent"))
  (if _returnvalue
    (bind (_bblockinghit _binitialoverlap _time _distance _location _impactpoint _normal _impactnormal _physmat _hitactor) (`GameplayStatics.BreakHitResult` _outhit))
    (`KismetSystemLibrary.PrintString` (`KismetSystemLibrary.GetDisplayName` _hitactor))
    (bind _returnvalue_2 (`GameplayStatics.SpawnEmitterAttached` (`self.LaserParticle`) (`Actor.RootComponent` (`self.GetOwner`))))
    (`|ExecutionSequence`
      (:`then_0`
        (`FXSystemComponent.SetActorParameter` _returnvalue_2 "BeamSource" (`self.GetOwner`)))
      (:`then_1`
        (`FXSystemComponent.SetActorParameter` _returnvalue_2 "BeamTarget" _hitactor))
      (:`then_2`
        (set `self.ParticleSystem` _returnvalue_2)))))

(fn `StopLaser`
  (bind _particlesystem (`self.ParticleSystem`))
  (`/Engine/EditorBlueprintResources/StandardMacros.IsValid` _particlesystem
    (:`Is Valid`
      (`self.K2_DestroyComponent` _particlesystem))))